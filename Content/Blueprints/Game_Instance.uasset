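; Game Instance Blueprint that handles hosting and joining multiplayer sessions, with optional LAN use.
; HostSeccion stores the player limit and creates a session with that many public connections for the first player controller.
; FindSession searches for sessions and issues a join on every result in a loop, with no filtering or selection.
; Outcomes are only printed to screen; the host path does no map travel.
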(event `HostSeccion`
  (params (MaxPlayers :type Integer) (UserLan :type Boolean))
  (bind _output_get (set `self.Max Players` MaxPlayers))
  (`CreateSessionCallbackProxy.CreateSession` (`GameplayStatics.GetPlayerController` 0) _output_get UserLan
    (:`OnSuccess`
      (`KismetSystemLibrary.PrintString` "?fctun"))
    (:`OnFailure`
      (`KismetSystemLibrary.PrintString` "error session"))))

(event `FindSession`
  (params (PlayerController :type "PlayerController Object Reference") (bUseLAN :type Boolean))
  (bind _results (`FindSessionsCallbackProxy.FindSessions` PlayerController 99999 bUseLAN)
    (:`OnSuccess`
      (for _array_element _results
        (`JoinSessionCallbackProxy.JoinSession` PlayerController _array_element
          (:`OnSuccess`
            (`KismetSystemLibrary.PrintString` "Success"))
          (:`OnFailure`
            (`KismetSystemLibrary.PrintString` "Failure" :!label _label)))))
    (:`OnFailure`
      (goto _label))))